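; NPC dialogue component that sets up a player interaction zone and turns speech bubbles toward the player's follow camera.
; AllowPlayerInteraction stores the approach flag and, when true, attaches a new 256-unit sphere to the NPC's capsule.
; Tick calls NPCToPlayerLineTrace, which performs no trace but re-calls that event while the flag is set, adding spheres repeatedly.
; SphereDetection is unwired, and the BP_NPC owner cast is unused.
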(event Custom|SpeechBubbleFacesPlayer
  (params (DialogBubble :type Widget%20Component%20Object%20Reference))
  (bind _returnvalue (Actor|GetActorOfClass "/Game/ThirdPerson/Blueprints/BP_KOW_Character.BP_KOW_Character_C"))
  (Transformation|SetWorldRotation DialogBubble (Math|Rotator|FindLookatRotation (Transformation|GetWorldLocation DialogBubble) (Transformation|GetWorldLocation (Variables|/Game/ThirdPerson/Blueprints/BP_KOW_Character.BP_KOW_Character_C|GetFollowCamera _returnvalue))) false false))

(event Custom|Allow%20Player%20Interaction
  (params (InteractWithPlayer :type Boolean))
  (bind _asbp_npc (Utilities|NPCBlueprintClass))
  (Variables|Default|SetbPlayerCanApproach InteractWithPlayer)
  (if (Variables|Default|GetbPlayerCanApproach)
    (bind _returnvalue (Game|AddComponentbyClass _asbp_npc "/Script/Engine.SphereComponent" true (Transformation|GetActorTransform _asbp_npc)))
    (Transformation|AttachComponentToComponent _returnvalue (Variables|/Script/Engine.Character|GetCapsuleComponent _asbp_npc) "None" "KeepRelative" "KeepRelative" "KeepRelative" true)
    (Components|Sphere|SetSphereRadius _returnvalue 256.0 true)))

(event Custom|NPC%20to%20Player%20Line%20Trace
  (params (Player :type BP%20KOW%20Character%20Object%20Reference))
  (bind _bplayercanapproach (Variables|Default|GetbPlayerCanApproach))
  ;[1 0 0] DEBUG REquired
  (if _bplayercanapproach
    (CallFunction|AllowPlayerInteraction _bplayercanapproach)))

(event EventTick
  (params (DeltaSeconds :type Float%20%28single-precision%29))
  (CallFunction|NPCtoPlayerLineTrace))
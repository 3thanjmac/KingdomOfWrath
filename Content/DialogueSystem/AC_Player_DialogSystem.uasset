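; Player dialogue component that toggles an NPC conversation with the F key.
; Starting spawns and possesses a camera offset from the player, freezes movement and look input, and triggers the NPC component's lines, voice-over and conversation display.
; Ending restores the player camera, input and velocity saved at BeginPlay.
; Player and NPC are looked up by class, so the first BP_NPC found is used; the proximity check only prints its result.
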(event Custom|HideConversation
  (CallFunction|ShowHideConversation false))

(event Custom|AddConversationCamera
  ;[1 1 1] Changing camera location
  (bind _returnvalue (Game|SpawnActorfromClass "/Game/DialogueSystem/BP_DialogSpector.BP_DialogSpector_C" (Math|Transform|MakeTransform (+ (.location (Transformation|GetWorldTransform (Variables|/Script/Engine.Actor|GetRootComponent (CallFunction|GetKOW)))) "40.000000,-174.000000,50.000000") "-4.000000,125.000000,0.000000" "1.000000,1.000000,1.000000") "AlwaysSpawn" "MultiplyWithRoot" 0 0))
  (Variables|Default|SetSpawnDialogCamera _returnvalue)
  (CallFunction|PossesDialogCamera))

(event Custom|ResetCamera
  ;[1 1 1] Changing camera location
  (CallFunction|PossesPlayerCamera))

(event Custom|Check%20If%20player%20is%20still%20within%20the%20NPC%20collision
  (params (NPC :type Actor%20Object%20Reference) (Max%20Distance :type Float%20%28double-precision%29))
  (bind _returnvalue (CallFunction|CharacterDetection NPC (CallFunction|GetKOW) Max%20Distance))
  (Development|PrintString (Utilities|String|ToString(Boolean) _returnvalue)))

(event Custom|Freeze%20Player%20Movement
  (bind _returnvalue (Game|GetPlayerController 0))
  (bind _returnvalue_2 (Pawn|GetControlledPawn _returnvalue))
  (bind _returnvalue_3 (Pawn|GetController _returnvalue_2))
  ;[1 1 1] Freeze the player when they are talking to npc
  (Variables|/Script/Engine.MovementComponent|SetVelocity (Variables|/Script/Engine.Character|GetCharacterMovement (CallFunction|GetKOW)) "0, 0, 0")
  (Input|SetIgnoreLookInput _returnvalue_3 true)
  (Input|SetIgnoreMoveInput _returnvalue_3 true))

(event Custom|UnfreezePlayer
  (bind _returnvalue (Game|GetPlayerController 0))
  (bind _returnvalue_2 (Pawn|GetControlledPawn _returnvalue))
  (bind _returnvalue_3 (Pawn|GetController _returnvalue_2))
  ;[1 1 1] Freeze the player when they are talking to npc
  (Variables|/Script/Engine.MovementComponent|SetVelocity (Variables|/Script/Engine.Character|GetCharacterMovement (CallFunction|GetKOW)) (Variables|DialogSystem|GetStartingVelocity))
  (Input|SetIgnoreLookInput _returnvalue_3 false)
  (Input|SetIgnoreMoveInput _returnvalue_3 false))

(event Custom|ShowConversation
  (CallFunction|ShowHideConversation true))

(event EventBeginPlay
  (bind _returnvalue (Actor|GetActorOfClass "/Game/ThirdPerson/Blueprints/BP_CameraManager.BP_CameraManager_C"))
  (Variables|Default|SetcamManager _returnvalue)
  (if (not (Variables|DialogSystem|GetbIsItTheWindsOfMorrow))
    (Variables|DialogSystem|SetStartingVelocity (Variables|/Script/Engine.MovementComponent|GetVelocity (Variables|/Script/Engine.Character|GetCharacterMovement (CallFunction|GetKOW))))))

(event Input|KeyboardEvents|F
  (params (Key :type Key%20Structure :default "None"))
  ;[1 1 1] Initiate Conversation
  (:Pressed
    (Utilities|FlowControl|FlipFlop
      (:A
        (CallFunction|AddConversationCamera)
        (Default|DisplayLines (Variables|/Game/ThirdPerson/Enemies/BP_NPC.BP_NPC_C|GetAC_NPC_DialogSystem (CallFunction|GetNPC)))
        (CallFunction|ShowConversation)
        (CallFunction|FreezePlayerMovement)
        (Default|PlayCustomVO (Variables|/Game/ThirdPerson/Enemies/BP_NPC.BP_NPC_C|GetAC_NPC_DialogSystem (CallFunction|GetNPC))))
      (:B
        (CallFunction|ResetCamera)
        (CallFunction|HideConversation)
        (CallFunction|UnfreezePlayer)))))

(fn GetKOW
  (bind _returnvalue (Actor|GetActorOfClass "/Game/ThirdPerson/Blueprints/BP_KOW_Character.BP_KOW_Character_C"))
  (return _returnvalue))

(fn GetNPC
  (bind _returnvalue (Actor|GetActorOfClass "/Game/ThirdPerson/Enemies/BP_NPC.BP_NPC_C"))
  (return _returnvalue))

(fn GetAllUniqueNPCs
  (bind _outactors (Actor|GetAllActorsOfClass "/Game/ThirdPerson/Enemies/BP_NPC.BP_NPC_C"))
  (return _outactors))
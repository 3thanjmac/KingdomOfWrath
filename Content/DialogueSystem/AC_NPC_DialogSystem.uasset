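; NPC dialogue component that manages an NPC's dialogue window, lines and voice-over.
; BeginPlay creates the hidden window and sets the speaker name; separate events show or hide it and turn a speech bubble toward the player camera.
; DisplayLines fetches the current dialogue row, displays it and stores its sound, which PlayCustomVO plays when a proximity check passes.
; Interaction gating is a stub, and several proximity and NPC-registration fragments are unwired.
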(event Custom|Show%20Interaction
  (bind _returnvalue (Components|GetOwner))
  (Widget|SetVisibility (Variables|Default|GetDial) "Visible")
  (CallFunction|ShowHideInteraction true)
  (bind _outactors (CallFunction|GetInteractiveNPC _returnvalue))
  (Development|PrintString (Utilities|GetDisplayName (Utilities|Array|Get(acopy) _outactors (Utilities|Array|FindItem _outactors _returnvalue)))))

(event Custom|Hide%20Interaction
  (Widget|SetVisibility (Variables|Default|GetDial) "Hidden")
  (CallFunction|ShowHideInteraction false))

(event Custom|Allow%20Player%20Interaction
  (params (InteractWithPlayer :type Boolean))
  (Variables|Default|SetbPlayerCanApproach InteractWithPlayer)
  (if (Variables|Default|GetbPlayerCanApproach)
    _))

(event Custom|NPC%20to%20Player%20Line%20Trace
  (params (Player :type BP%20KOW%20Character%20Object%20Reference))
  (bind _bplayercanapproach (Variables|Default|GetbPlayerCanApproach))
  ;[1 0 0] DEBUG REquired
  (if _bplayercanapproach
    (CallFunction|AllowPlayerInteraction _bplayercanapproach)))

(event Custom|SetCharacterName
  (Default|AddSpeakerEvent (Variables|/Game/DialogueSystem/Dialog_Widget/W_DialogueMainWindow.W_DialogueMainWindow_C|GetW_InteractionDialogWindow (Variables|Default|GetDial)) (Utilities|Text|ToText(String) (.charactername (Variables|DialogSystemPerimeters|GetNPC_Information)))))

(event Custom|SpeechBubbleFacesPlayer
  (params (DialogBubble :type Widget%20Component%20Object%20Reference))
  (bind _returnvalue (Actor|GetActorOfClass "/Game/ThirdPerson/Blueprints/BP_KOW_Character.BP_KOW_Character_C"))
  (Variables|Default|SetKOW_Ref _returnvalue)
  (Transformation|SetWorldRotation DialogBubble (Math|Rotator|FindLookatRotation (Transformation|GetWorldLocation DialogBubble) (Transformation|GetWorldLocation (Variables|/Game/ThirdPerson/Blueprints/BP_KOW_Character.BP_KOW_Character_C|GetFollowCamera _returnvalue))) false false))

(event Custom|DisplayLines
  (bind (_character_name _text_and_vo) (CallFunction|SetDialogParagraph (.currentinteractiverowname (Variables|DialogSystemPerimeters|GetNPC_Information))))
  (Default|AddNameandLineEvent (Variables|Default|GetDial) (Utilities|Text|ToText(String) _character_name) (Utilities|Text|ToText(String) (.dialog_text _text_and_vo)))
  (Variables|Default|SetRegisteredSound (.dialog_sound _text_and_vo)))

(event Custom|Play%20Custom%20VO
  (bind _returnvalue (CallFunction|CharacterDetection (Components|GetOwner self) (Variables|Default|GetKOW_Ref) 2e+02))
  (if _returnvalue
    (Audio|PlaySound2D (Variables|Default|GetRegisteredSound) 1.0 1.0 0.0 0 0)))

(event EventBeginPlay
  (CallFunction|SetCharacterName)
  (bind _dialogmainwindow (CallFunction|OpenMainDialogWindow))
  (bind _output_get (Variables|Default|SetDial _dialogmainwindow))
  (UserInterface|Viewport|AddtoViewport _output_get 0)
  (Widget|SetVisibility _output_get "Hidden"))

(fn GetAllUniqueNPCs
  (return 0))